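; BP_UIController manages the flight display widget and intruder traffic, adding detect-and-avoid threat bands.
; It creates and toggles WBP_UIDesign_19 and spawns BP_IntruderController actors, activating only the first with table data.
; UpdateUI refreshes intruders, then passes scaled ownship and closest-intruder states to SimHUD's circle-intersection solver.
; The resulting band angles and threat level are logged to CSV and fed to the widget, except on UseLast updates, which only refresh intruders.
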(fn ConstructionScript)

(fn SetUI
  (params (Selection :type Integer))
  (if (Utilities|IsValid (Variables|Default|GetActiveUIObject))
    (Default|Disable (Variables|Default|GetActiveUI)))
  (switch int Selection
    (:0
      _)
    (:1
      _))
  (bind _returnvalue (UserInterface|CreateWidget "/Game/Custom/WBP_UIDesign_19.WBP_UIDesign_19_C" (Game|GetPlayerController 0)))
  (Variables|Default|SetActiveUI _returnvalue)
  (UserInterface|Viewport|AddtoViewport _returnvalue 0)
  (Variables|Default|SetActiveUIObject _returnvalue)
  (Variables|/Script/UMG.Widget|SetVisibility _returnvalue "Hidden"))

(fn ToggleUI
  (params (SetUI :type Boolean))
  (bind _activeuiobject (Variables|Default|GetActiveUIObject))
  (if (Utilities|IsValid (Variables|Default|GetActiveUIObject))
    (if (or (Widget|IsVisible _activeuiobject) SetUI)
      (Widget|SetVisibility _activeuiobject "Hidden")
      (else
        (Widget|SetVisibility _activeuiobject "Visible")))))

(fn UpdateUI
  (params (OwnshipHeading :type Float%20%28double-precision%29) (OwnshipLat :type Float%20%28double-precision%29) (OwnshipLong :type Float%20%28double-precision%29) (OwnshipAltitude :type Float%20%28double-precision%29) (OwnshipGroundSpeed :type Float%20%28double-precision%29) (OwnshipRoll :type Float%20%28double-precision%29) (OwnshipPitch :type Float%20%28double-precision%29) (FlightTime :type Float%20%28double-precision%29) (Intruders :type Array%20of%20BP%20Intruder%20Object%20References) (TopLeftCoord :type Vector) (TopRightCoord :type Vector) (BottomRightCoord :type Vector) (BottomLeftCoord :type Vector) (Debug :type Boolean) (UseLast :type Boolean))
  (bind _addition_var (Variables|Default|Getaddition%20var))
  (bind _multiply_var (Variables|Default|Getmultiply%20var))
  (if (Utilities|IsValid (Variables|Default|GetActiveUIObject))
    (if (Utilities|IsValid (Variables|Default|GetIntruderController))
      (if (not UseLast)
        (CallFunction|UpdateIntruder TopLeftCoord TopRightCoord BottomRightCoord OwnshipAltitude false)
        ;[1 1 1] DAIDULUS
        (if (< OwnshipGroundSpeed 1e+01)
          (Variables|Default|SetOwnship%20speed%20multiplier 1e+02)
          (elif (and (>= OwnshipGroundSpeed 1e+01) (< OwnshipGroundSpeed 1e+02))
            (Variables|Default|SetOwnship%20speed%20multiplier 1e+01)))
        (bind _returnvalue (Actor|GetActorOfClass "/Script/CesiumRuntime.CesiumGeoreference"))
        (if (> OwnshipHeading 1.8e+02)
          (Variables|Default|SetOwnship%20heading%20Var (- OwnshipHeading 3.6e+02))
          (else
            (Variables|Default|SetOwnship%20heading%20Var OwnshipHeading)))
        (bind (_intruderheading _intruderdistance _foundintruder _intruderloc) (Default|GetClosestIntruderData (Variables|Default|GetIntruderController) (Math|Vector|MakeVector OwnshipLong OwnshipLat OwnshipAltitude))) ; Gets closest intruder and returns its heading and distance for now -- later will return relevant data for daidalus
        (if (> _intruderheading 1.8e+02)
          (Variables|Default|SetIntruder%20heading%20Var (- _intruderheading 3.6e+02))
          (else
            (Variables|Default|SetIntruder%20heading%20Var _intruderheading)))
        (bind _returnvalue_2 (Actor|GetActorOfClass "/Script/CesiumRuntime.CesiumGeoreference"))
        ;[1 1 1] New DAA
        (bind _returnvalue_3 (Actor|GetActorOfClass "/Script/AirSim.SimHUD"))
        (bind _structout (Utilities|Struct|SetmembersinAircraft (Utilities|Struct|MakeAircraft -5e+01 0.0) (* OwnshipLat _multiply_var) (* OwnshipLong _multiply_var) (+ (* OwnshipGroundSpeed (Variables|Default|GetOwnship%20speed%20multiplier)) (Variables|Default|Getadd%20speed%20var)) (Variables|Default|GetOwnship%20heading%20Var) (Utilities|Array|MakeArray 0.0)))
        (bind _structout_2 (Utilities|Struct|SetmembersinAircraft (Utilities|Struct|MakeAircraft -5e+01 0.0) (+ (* (.Y (Math|Vector|BreakVector _intruderloc)) _multiply_var) _addition_var) (+ (* (.X (Math|Vector|BreakVector _intruderloc)) _multiply_var) _addition_var) (Variables|Default|GetIntruder%20Speed%20Var) (Variables|Default|GetIntruder%20heading%20Var) (Utilities|Array|MakeArray 0.0)))
        (bind _structout_3 (Utilities|Struct|SetmembersinNewParameters (Utilities|Struct|MakeNewParameters 2e+03 8e+03 8e+03 1.2e+04) 3.7 3.7 5.0 5.0))
        (bind (_startangle _endangle _level _distance) (Class|SimHUD|FindIntersectionwithCircle _returnvalue_3 _structout_3 _structout _structout_2))
        (Class|SimHUD|SaveDataIntoCsvFile _returnvalue_3 (Variables|Default|GetFirstTimeEntryVar) (Math|Vector|MakeVector (.x (Utilities|Struct|BreakAircraft _structout)) (.y (Utilities|Struct|BreakAircraft _structout)) _distance) "0, 0, 0" (Variables|Default|GetOwnship%20heading%20Var) OwnshipGroundSpeed (Math|Vector|MakeVector (.x (Utilities|Struct|BreakAircraft _structout_2)) (.y (Utilities|Struct|BreakAircraft _structout_2)) (Variables|Default|GetIntruder%20heading%20Var)) "0, 0, 0" (Variables|Default|GetIntruder%20heading%20Var) _distance _startangle _endangle _level)
        (Variables|Default|SetFirstTimeEntryVar 0)
        (Default|UpdateUI (Variables|Default|GetActiveUI) OwnshipHeading OwnshipAltitude OwnshipGroundSpeed OwnshipRoll OwnshipPitch FlightTime (+ _startangle 0.0) (+ _endangle 0.0) _level Intruders TopLeftCoord TopRightCoord BottomRightCoord BottomLeftCoord Debug :!label _label)
        (else
          (CallFunction|UpdateIntruder TopLeftCoord TopRightCoord BottomRightCoord OwnshipAltitude true)))
      (else
        (goto _label)))))

(fn AddIntruderData
  (params (IntruderTable :type Data%20Table%20Object%20Reference) (IntruderTable2 :type Data%20Table%20Object%20Reference))
  (bind _returnvalue (Math|Transform|MakeTransform "0, 0, 0"))
  (Utilities|FlowControl|Sequence
    (:then_0
      (bind _returnvalue_2 (Game|SpawnActorfromClass "/Game/Custom/BP_IntruderController.BP_IntruderController_C" _returnvalue "Undefined" "MultiplyWithRoot" 0 0))
      (bind _output_get (Variables|Default|SetIntruderController _returnvalue_2))
      (Default|Activate _output_get IntruderTable))
    (:then_1
      (bind _returnvalue_3 (Game|SpawnActorfromClass "/Game/Custom/BP_IntruderController.BP_IntruderController_C" _returnvalue "Undefined" "MultiplyWithRoot" 0 0))
      (Variables|Default|SetIntruderController_1 _returnvalue_3))))

(fn UpdateIntruder
  (params (TopLeftCoords :type Vector) (TopRightCoords :type Vector) (BottomRightCoords :type Vector) (OwnshipAltitude :type Float%20%28double-precision%29) (UseLast :type Boolean))
  (bind _intrudercontroller (Variables|Default|GetIntruderController))
  (if (Utilities|IsValid _intrudercontroller)
    (Default|Update _intrudercontroller TopLeftCoords TopRightCoords BottomRightCoords OwnshipAltitude UseLast)))

(fn FakeDAIDALUS
  (params (IntruderHeading :type Float%20%28double-precision%29) (IntruderDistance :type Float%20%28double-precision%29))
  (return (- IntruderHeading 25.0) (+ IntruderHeading 25.0) 2))

(fn SetStartandEndAngles
  (params (InStartAngle :type Float%20%28double-precision%29) (InEndAngle :type Float%20%28double-precision%29) (intruder%20loc :type Vector) (ownship%20loc :type Vector))
  (if (<= (+ InStartAngle InEndAngle) -1.8e+02)
    (Development|PrintString (Utilities|String|ToString(Vector) intruder%20loc))
    (Development|PrintString (Utilities|String|ToString(Vector) ownship%20loc))
    (return 0.0 0.0)))